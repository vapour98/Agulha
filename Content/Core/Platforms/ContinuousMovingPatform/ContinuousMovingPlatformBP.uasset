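; Moving platform that travels between two configurable points and carries BP_Lappe along with it.
; The construction script feeds Point1 and Point2 into InterpToMovement as relative control points and sets its Duration.
; Box overlap attaches BP_Lappe's root component to the Box, keeping world transform.
; End overlap detaches whichever actor leaves, without a type check.
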(event OnComponentBeginOverlap(Box)
  (params (OverlappedComponent :type Primitive%20Component%20Object%20Reference) (OtherActor :type Actor%20Object%20Reference) (OtherComp :type Primitive%20Component%20Object%20Reference) (OtherBodyIndex :type Integer) (bFromSweep :type Boolean) (SweepResult :type Hit%20Result%20Structure%20%28by%20ref%29))
  (bind _asbp_lappe (Utilities|Casting|CastToBP_Lappe OtherActor))
  (Transformation|AttachComponentToComponent (Variables|/Script/Engine.Actor|GetRootComponent _asbp_lappe) (Variables|Default|GetBox) "None" "KeepWorld" "KeepWorld" "KeepWorld" true))

(event OnComponentEndOverlap(Box)
  (params (OverlappedComponent :type Primitive%20Component%20Object%20Reference) (OtherActor :type Actor%20Object%20Reference) (OtherComp :type Primitive%20Component%20Object%20Reference) (OtherBodyIndex :type Integer))
  (Transformation|DetachFromActor OtherActor "KeepWorld" "KeepWorld" "KeepWorld"))

(event EventBeginPlay)

(event Collision|EventActorBeginOverlap
  (params (OtherActor :type Actor%20Object%20Reference)))

(event EventTick
  (params (DeltaSeconds :type Float%20%28single-precision%29)))

(fn ConstructionScript
  (bind _interptomovement (Variables|Default|GetInterpToMovement))
  (Variables|/Script/Engine.InterpToMovementComponent|SetControlPoints _interptomovement (Utilities|Array|MakeArray (Utilities|Struct|MakeInterpControlPoint (Variables|Default|GetPoint1) true) (Utilities|Struct|MakeInterpControlPoint (Variables|Default|GetPoint2) true)))
  (Variables|/Script/Engine.InterpToMovementComponent|SetDuration _interptomovement (Variables|Default|GetDuration)))