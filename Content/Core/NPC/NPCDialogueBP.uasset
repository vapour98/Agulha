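; NPC actor that shows a prompt and runs multi-line dialogue when BP_Lappe is nearby.
; Box overlap reveals the TextRender and creates the DialogueWidget; leaving hides the text and removes the widget.
; The DilogueOccurs event passes NPCText to the widget, reveals its image and text, then advances TextRow or removes the widget at the array's end.
; A DoOnce gates each step and resets immediately afterward via ResetDialogue.
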(event OnComponentBeginOverlap(Box)
  (params (OverlappedComponent :type Primitive%20Component%20Object%20Reference) (OtherActor :type Actor%20Object%20Reference) (OtherComp :type Primitive%20Component%20Object%20Reference) (OtherBodyIndex :type Integer) (bFromSweep :type Boolean) (SweepResult :type Hit%20Result%20Structure%20%28by%20ref%29))
  (Utilities|Casting|CastToBP_Lappe OtherActor)
  (Development|SetHiddeninGame (Variables|Default|GetTextRender) false false)
  (bind _returnvalue (UserInterface|CreateWidget "/Game/Core/NPC/DialogueWidget.DialogueWidget_C"))
  (bind _output_get (Variables|Default|SetDialogueUI _returnvalue))
  (UserInterface|Viewport|AddtoViewport _output_get 0))

(event OnComponentEndOverlap(Box)
  (params (OverlappedComponent :type Primitive%20Component%20Object%20Reference) (OtherActor :type Actor%20Object%20Reference) (OtherComp :type Primitive%20Component%20Object%20Reference) (OtherBodyIndex :type Integer))
  (bind _dialogueui (Variables|Default|GetDialogueUI))
  (Utilities|Casting|CastToBP_Lappe OtherActor)
  (Development|SetHiddeninGame (Variables|Default|GetTextRender) true false)
  (Utilities|IsValid _dialogueui
    (:Is%20Valid
      (Widget|RemovefromParent _dialogueui))))

(event Custom|ResetDialogue
  (bind _dialogueui (Variables|Default|GetDialogueUI))
  (bind _dialogueui_2 (Variables|Default|GetDialogueUI))
  (Utilities|FlowControl|DoOnce false) ; enters at Reset
)

(event EventBeginPlay)

(event Collision|EventActorBeginOverlap
  (params (OtherActor :type Actor%20Object%20Reference)))

(event EventDilogueOccurs
  (bind _dialogueui (Variables|Default|GetDialogueUI))
  (bind _dialogueui_2 (Variables|Default|GetDialogueUI))
  (Utilities|FlowControl|DoOnce false
    (:Completed
      (Variables|/Game/Core/NPC/DialogueWidget.DialogueWidget_C|SetText _dialogueui_2 (Variables|Default|GetNPCText))
      (Widget|SetVisibility (Variables|/Game/Core/NPC/DialogueWidget.DialogueWidget_C|GetImage_0 _dialogueui_2) "Visible")
      (if (> (+ (Variables|/Game/Core/NPC/DialogueWidget.DialogueWidget_C|GetTextRow (Variables|Default|GetDialogueUI)) 1) (- (Utilities|Array|Length (Variables|Default|GetNPCText)) 1))
        (Widget|RemovefromParent _dialogueui)
        (CallFunction|ResetDialogue)
        (else
          (Variables|/Game/Core/NPC/DialogueWidget.DialogueWidget_C|SetTextRow _dialogueui (+ (Variables|/Game/Core/NPC/DialogueWidget.DialogueWidget_C|GetTextRow (Variables|Default|GetDialogueUI)) 1))
          (CallFunction|ResetDialogue))))))

(fn ConstructionScript)