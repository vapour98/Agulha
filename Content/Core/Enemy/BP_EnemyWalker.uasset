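; Enemy walker that patrols back and forth along the world Y axis and damages the BP_Lappe player on contact.
; BeginPlay converts bound offsets to world positions; Tick applies movement input and flips direction at either bound.
; Capsule hits apply enemy damage unless BeenHit is set.
; That flag gives a brief invulnerability window via a delay, skipped when GameInstanceTest health is one or less.
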(event OnComponentHit(CapsuleComponent)
  (params (HitComponent :type Primitive%20Component%20Object%20Reference) (OtherActor :type Actor%20Object%20Reference) (OtherComp :type Primitive%20Component%20Object%20Reference) (NormalImpulse :type Vector :default "0, 0, 0") (Hit :type Hit%20Result%20Structure%20%28by%20ref%29))
  (Utilities|HitPlayer OtherActor))

(event EventBeginPlay
  (bind _capsulecomponent (Variables|Default|GetCapsuleComponent))
  (bind _returnvalue (Transformation|GetWorldLocation _capsulecomponent))
  (Variables|Default|SetStartBound (+ _returnvalue (Variables|Default|GetStartBound)))
  (Variables|Default|SetEndBound (+ _returnvalue (Variables|Default|GetEndBound))))

(event Collision|EventActorBeginOverlap
  (params (OtherActor :type Actor%20Object%20Reference)))

(event EventTick
  (params (DeltaSeconds :type Float%20%28single-precision%29))
  (Utilities|FlowControl|Sequence
    (:then_0
      (Pawn|Input|AddMovementInput "0,0.250000, 0" (select (Variables|Default|GetbMoveRight) -1.0 1.0) false))
    (:then_1
      (Utilities|CheckLocation))))

(fn ConstructionScript
  (|CallParentFunction))