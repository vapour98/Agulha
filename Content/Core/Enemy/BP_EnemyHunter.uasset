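; Enemy that patrols along the Y axis between StartBound and EndBound, chasing BP_Lappe at stronger movement input while it overlaps Sphere1.
; Tick drives movement and the bounds check, which flips patrol direction and drops the chase at either edge.
; Capsule hits apply enemy damage unless BeenHit is set, a half-second flag on the player that is only raised when GameInstanceTest health exceeds one.
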(event OnComponentHit(CapsuleComponent)
  (params (HitComponent :type Primitive%20Component%20Object%20Reference) (OtherActor :type Actor%20Object%20Reference) (OtherComp :type Primitive%20Component%20Object%20Reference) (NormalImpulse :type Vector :default "0, 0, 0") (Hit :type Hit%20Result%20Structure%20%28by%20ref%29))
  (Utilities|HitPlayer OtherActor))

(event OnComponentBeginOverlap(Sphere1)
  (params (OverlappedComponent :type Primitive%20Component%20Object%20Reference) (OtherActor :type Actor%20Object%20Reference) (OtherComp :type Primitive%20Component%20Object%20Reference) (OtherBodyIndex :type Integer) (bFromSweep :type Boolean) (SweepResult :type Hit%20Result%20Structure%20%28by%20ref%29))
  (bind _asbp_lappe (Utilities|Casting|CastToBP_Lappe OtherActor))
  (Variables|Default|SetTracker _asbp_lappe)
  (Variables|Default|SetbFoundPlayer true))

(event OnComponentEndOverlap(Sphere1)
  (params (OverlappedComponent :type Primitive%20Component%20Object%20Reference) (OtherActor :type Actor%20Object%20Reference) (OtherComp :type Primitive%20Component%20Object%20Reference) (OtherBodyIndex :type Integer))
  (Utilities|Casting|CastToBP_Lappe OtherActor)
  (Variables|Default|SetbFoundPlayer false))

(event EventBeginPlay)

(event Collision|EventActorBeginOverlap
  (params (OtherActor :type Actor%20Object%20Reference)))

(event EventTick
  (params (DeltaSeconds :type Float%20%28single-precision%29))
  (Utilities|FlowControl|Sequence
    (:then_0
      (if (Variables|Default|GetbFoundPlayer)
        (Pawn|Input|AddMovementInput "0,0.500000, 0" (select (> (.y (Transformation|GetActorLocation)) (.y (Transformation|GetWorldLocation (Variables|/Script/Engine.Actor|GetRootComponent (Variables|Default|GetTracker))))) -1.0 1.0) false)
        (else
          (Utilities|AutoMove))))
    (:then_1
      (Utilities|CheckLocation))))

(fn ConstructionScript
  (|CallParentFunction))