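; BP_EnemyBat is a bat enemy that patrols back and forth along the world Y axis.
; Each tick adds movement input along Y, with the MoveRight flag setting the direction.
; A capsule hit flips that flag when the other actor is not the player pawn and the hit normal has a nonzero Y component.
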(event OnComponentHit(CapsuleComponent)
  (params (HitComponent :type Primitive%20Component%20Object%20Reference) (OtherActor :type Actor%20Object%20Reference) (OtherComp :type Primitive%20Component%20Object%20Reference) (NormalImpulse :type Vector :default "0, 0, 0") (Hit :type Hit%20Result%20Structure%20%28by%20ref%29))
  (if (!= OtherActor (Game|Player|GetPlayerPawn 0))
    (if (!= (.Y (Math|Vector|BreakVector (.normal Hit))) 0.0)
      (Variables|Default|SetbMoveRight (not (Variables|Default|GetbMoveRight))))))

(event EventBeginPlay)

(event Collision|EventActorBeginOverlap
  (params (OtherActor :type Actor%20Object%20Reference)))

(event EventTick
  (params (DeltaSeconds :type Float%20%28single-precision%29))
  (Pawn|Input|AddMovementInput "0.000000,2.000000, 0" (select (Variables|Default|GetbMoveRight) 1.0 -1.0) false))

(fn ConstructionScript
  (|CallParentFunction))