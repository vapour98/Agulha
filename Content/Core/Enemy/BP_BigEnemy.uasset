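; BP_BigEnemy is a large chasing enemy that moves along negative Y while the game instance's CanWallJump flag is true.
; BeginPlay turns its start, slow and end offsets into world positions.
; Tick drives movement, halving input once past the slow point and destroying the actor past the end point.
; Overlapping BP_Lappe with its Box deals massive chase damage, then resets the enemy to its start at normal speed.
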(event OnComponentBeginOverlap(Box)
  (params (OverlappedComponent :type Primitive%20Component%20Object%20Reference) (OtherActor :type Actor%20Object%20Reference) (OtherComp :type Primitive%20Component%20Object%20Reference) (OtherBodyIndex :type Integer) (bFromSweep :type Boolean) (SweepResult :type Hit%20Result%20Structure%20%28by%20ref%29))
  (bind _asbp_lappe (Utilities|Casting|CastToBP_Lappe OtherActor))
  (Game|Damage|ApplyDamage _asbp_lappe 1e+03 0 0 "/Game/Core/Enemy/DamageTypeChase.DamageTypeChase_C")
  (Transformation|SetWorldLocation (Variables|Default|GetCapsuleComponent) (Variables|Default|GetStartPoint) false false)
  (Variables|Default|SetSlowtime false))

(event EventBeginPlay
  (bind _capsulecomponent (Variables|Default|GetCapsuleComponent))
  (bind _returnvalue (Transformation|GetWorldLocation _capsulecomponent))
  (Variables|Default|SetStartPoint (+ (Variables|Default|GetStartPoint) _returnvalue))
  (Variables|Default|SetSlowPoint (+ (Variables|Default|GetSlowPoint) _returnvalue))
  (Variables|Default|SetEndPoint (+ (Variables|Default|GetEndPoint) _returnvalue)))

(event Collision|EventActorBeginOverlap
  (params (OtherActor :type Actor%20Object%20Reference)))

(event EventTick
  (params (DeltaSeconds :type Float%20%28single-precision%29))
  (bind _asgame_instance_test (Utilities|Casting|CastToGameInstanceTest (Game|GetGameInstance)))
  (if (Variables|/Game/GameInstance/GameInstanceTest.GameInstanceTest_C|GetbCanWallJump _asgame_instance_test)
    (Utilities|FlowControl|Sequence
      (:then_0
        (Utilities|FlowControl|Delay 0.2))
      (:then_1
        (Pawn|Input|AddMovementInput "0,-1.000000, 0" (select (Variables|Default|GetSlowtime) 0.25 0.5) false))
      (:then_2
        (if (< (.y (Transformation|GetWorldLocation (Variables|Default|GetCapsuleComponent))) (.y (Variables|Default|GetSlowPoint)))
          (Variables|Default|SetSlowtime true)))
      (:then_3
        (if (< (.y (Transformation|GetWorldLocation (Variables|Default|GetCapsuleComponent))) (.y (Variables|Default|GetEndPoint)))
          (Actor|DestroyActor))))))

(fn ConstructionScript
  (|CallParentFunction))