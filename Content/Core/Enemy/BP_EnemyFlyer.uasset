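; Flying enemy that patrols a Y/Z box defined relative to its spawn point and damages BP_Lappe on contact.
; Tick either auto-moves or steers toward the player while it is inside Sphere1; reaching a bound reverses patrol direction and drops the chase.
; Capsule hits damage a player not already flagged BeenHit, setting that flag if health exceeds one.
; Non-player hits set patrol direction from axis-aligned impact normals.
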(event OnComponentBeginOverlap(Sphere1)
  (params (OverlappedComponent :type Primitive%20Component%20Object%20Reference) (OtherActor :type Actor%20Object%20Reference) (OtherComp :type Primitive%20Component%20Object%20Reference) (OtherBodyIndex :type Integer) (bFromSweep :type Boolean) (SweepResult :type Hit%20Result%20Structure%20%28by%20ref%29))
  (bind _asbp_lappe (Utilities|Casting|CastToBP_Lappe OtherActor))
  (Variables|Default|SetTracker _asbp_lappe)
  (Variables|Default|SetbFoundPlayer true))

(event OnComponentEndOverlap(Sphere1)
  (params (OverlappedComponent :type Primitive%20Component%20Object%20Reference) (OtherActor :type Actor%20Object%20Reference) (OtherComp :type Primitive%20Component%20Object%20Reference) (OtherBodyIndex :type Integer))
  (Variables|Default|SetbFoundPlayer false))

(event OnComponentHit(CapsuleComponent)
  (params (HitComponent :type Primitive%20Component%20Object%20Reference) (OtherActor :type Actor%20Object%20Reference) (OtherComp :type Primitive%20Component%20Object%20Reference) (NormalImpulse :type Vector :default "0, 0, 0") (Hit :type Hit%20Result%20Structure%20%28by%20ref%29))
  (bind (_x _y _z) (Math|Vector|BreakVector (.impactnormal Hit)))
  (Utilities|HitPlayer OtherActor
    (:Out
      (if (== _z 1.0)
        (Variables|Default|SetbMoveUp false)
        (elif (== _z -1.0)
          (Variables|Default|SetbMoveUp true)))
      (if (== _y 1.0)
        (Variables|Default|SetbMoveRight false)
        (elif (== _y -1.0)
          (Variables|Default|SetbMoveRight true))))))

(event EventBeginPlay
  (bind _returnvalue (Transformation|GetActorLocation))
  (Variables|Default|SetStartBound (+ _returnvalue (Variables|Default|GetStartBound)))
  (Variables|Default|SetEndBound (+ _returnvalue (Variables|Default|GetEndBound))))

(event Collision|EventActorBeginOverlap
  (params (OtherActor :type Actor%20Object%20Reference)))

(event EventTick
  (params (DeltaSeconds :type Float%20%28single-precision%29))
  (Utilities|FlowControl|Sequence
    (:then_0
      (if (Variables|Default|GetbFoundPlayer)
        (Pawn|Input|AddMovementInput "0,0.500000,0.000000" (select (> (.y (Transformation|GetActorLocation)) (.y (Transformation|GetActorLocation (Variables|Default|GetTracker)))) -1.0 1.0) false)
        (Pawn|Input|AddMovementInput "0, 0,0.500000" (select (> (.z (Transformation|GetActorLocation)) (.z (Transformation|GetActorLocation (Variables|Default|GetTracker)))) -1.0 1.0) false)
        (else
          (Utilities|AutoMove))))
    (:then_1
      (Utilities|CheckSideLocation))
    (:then_2
      (Utilities|CheckUpLocation))))

(fn ConstructionScript
  (|CallParentFunction))